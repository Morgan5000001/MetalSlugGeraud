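; Boss arena trigger that starts the boss fight when the player character enters its box.
; Each overlap flags the player as having reached the boss; a DoOnce then makes the boss damageable, starts its AI pattern, turns on Block collision and blends the view to this actor.
; ResetPatern makes the same boss calls, lifts the blocking and re-arms the DoOnce; the node returning the view to the player is unconnected.
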(event OnComponentBeginOverlap(Box)
  (params (OverlappedComponent :type Primitive%20Component%20Object%20Reference) (OtherActor :type Actor%20Object%20Reference) (OtherComp :type Primitive%20Component%20Object%20Reference) (OtherBodyIndex :type Integer) (bFromSweep :type Boolean) (SweepResult :type Hit%20Result%20Structure%20%28by%20ref%29))
  (bind _bossref (Variables|Default|GetBossRef))
  (bind _block (Variables|Default|GetBlock))
  (bind _asbp_third_person_character (Utilities|Casting|CastToBP_ThirdPersonCharacter OtherActor))
  (Variables|/Game/ThirdPerson/Blueprints/BP_ThirdPersonCharacter.BP_ThirdPersonCharacter_C|SetReachBoss? _asbp_third_person_character true)
  (Utilities|FlowControl|DoOnce false
    (:Completed
      (Variables|/Game/Blueprint/Boss/BP_Boss.BP_Boss_C|SetCanBeDammaged _bossref true)
      (Default|StartPatern (.AsAIC%20Boss (Utilities|Casting|CastToAIC_Boss (AI|GetAIController _bossref))) true)
      (Collision|SetCollisionResponsetoChannel _block "ECC_WorldDynamic" "ECR_Block")
      (Collision|SetCollisionResponsetoChannel _block "ECC_Pawn" "ECR_Block")
      (Game|Player|SetViewTargetwithBlend (Game|GetPlayerController 0) self 2.4 "VTBlend_Linear" 0.0 false))))

(event Custom|ResetPatern
  (bind _bossref (Variables|Default|GetBossRef))
  (bind _bossref_2 (Variables|Default|GetBossRef))
  (bind _block (Variables|Default|GetBlock))
  (bind _block_2 (Variables|Default|GetBlock))
  (Variables|/Game/Blueprint/Boss/BP_Boss.BP_Boss_C|SetCanBeDammaged _bossref true)
  (Default|StartPatern (.AsAIC%20Boss (Utilities|Casting|CastToAIC_Boss (AI|GetAIController _bossref))) true)
  (Collision|SetCollisionResponsetoChannel _block_2 "ECC_WorldDynamic" "ECR_Ignore")
  (Collision|SetCollisionResponsetoChannel _block_2 "ECC_Pawn" "ECR_Ignore")
  (Utilities|FlowControl|DoOnce false) ; enters at Reset
)

(event EventBeginPlay)

(event Collision|EventActorBeginOverlap
  (params (OtherActor :type Actor%20Object%20Reference)))

(event EventTick
  (params (DeltaSeconds :type Float%20%28single-precision%29)))

(fn ConstructionScript)
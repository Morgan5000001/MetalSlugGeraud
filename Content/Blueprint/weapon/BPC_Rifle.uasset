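; Rifle weapon Blueprint that hands itself to its player reference on BeginPlay to be equipped and provides automatic fire.
; Fire starts a looping timer, offset by a negative start delay to cancel the first wait, and EndFire clears it.
; Each shot spawns a BP_Projectile at ProjectileSpawn, setting its velocity along the player's input direction in the YZ plane, or actor forward without input.
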(event Custom|Shoot
  (bind _playerref (Variables|Default|GetplayerRef))
  (bind _action_value (Variables|/Game/ThirdPerson/Blueprints/BP_ThirdPersonCharacter.BP_ThirdPersonCharacter_C|GetAction%20Value _playerref))
  (bind (_x _y) (Math|Vector2D|BreakVector2D _action_value))
  (bind _returnvalue (Game|SpawnActorfromClass "/Game/Blueprint/Projectile/BP_Projectile.BP_Projectile_C" (Transformation|GetWorldTransform (Variables|Default|GetProjectileSpawn)) "Undefined" "MultiplyWithRoot" 0 1e+01 0))
  (Variables|/Script/Engine.MovementComponent|SetVelocity (Variables|/Game/Blueprint/Projectile/BP_Projectile.BP_Projectile_C|GetProjectileMovement _returnvalue) (* (select (and (== _x 0.0) (== _y 0.0)) (Transformation|GetActorForwardVector _playerref) (Math|Vector|Normalize (Math|Vector|MakeVector 0.0 _x _y))) 1.2e+03)))

(event EventFire
  (bind _returnvalue (Math|Float|MakeLiteralFloat 0.3))
  (bind _returnvalue_2 (Utilities|Time|SetTimerbyEvent (delegate Custom|Shoot) _returnvalue true (* _returnvalue -1.0)))
  (Variables|Default|SetFireTimer _returnvalue_2))

(event EventEndFire
  (Utilities|Time|ClearandInvalidateTimerbyHandle (Variables|Default|GetFireTimer)))

(event EventBeginPlay
  (bind _playerref (Variables|Default|GetplayerRef)
    (:then
      (Default|EquipWeapon _playerref self))
    (:else)))

(fn ConstructionScript
  (|CallParentFunction))
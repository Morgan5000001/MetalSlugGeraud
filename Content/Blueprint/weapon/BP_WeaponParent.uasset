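; BP_WeaponParent is a base weapon Blueprint that the player picks up by walking into its Box.
; On overlap with BP_ThirdPersonCharacter, it stores the player reference, adds itself uniquely to the character's WeaponsTab array and calls EquipWeapon, with a debug print in between.
; It then destroys the Box so that pickup cannot repeat.
; Fire, EndFire and HandleHaptics are empty events, apparently hooks for child weapons.
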(event OnComponentBeginOverlap(Box)
  (params (OverlappedComponent :type Primitive%20Component%20Object%20Reference) (OtherActor :type Actor%20Object%20Reference) (OtherComp :type Primitive%20Component%20Object%20Reference) (OtherBodyIndex :type Integer) (bFromSweep :type Boolean) (SweepResult :type Hit%20Result%20Structure%20%28by%20ref%29))
  (bind _asbp_third_person_character (Utilities|Casting|CastToBP_ThirdPersonCharacter OtherActor))
  (bind _output_get (Variables|Default|SetplayerRef _asbp_third_person_character))
  (Variables|Default|SetAs%20BP%20Third%20Person%20Character _output_get)
  (Utilities|Array|AddUnique (Variables|/Game/ThirdPerson/Blueprints/BP_ThirdPersonCharacter.BP_ThirdPersonCharacter_C|GetWeaponsTab _asbp_third_person_character) self)
  (Development|PrintString "88")
  (Default|EquipWeapon _asbp_third_person_character self)
  (Components|DestroyComponent (Variables|Default|GetBox)))

(event Custom|HandleHaptics)

(event Custom|Fire)

(event Custom|EndFire)

(event EventBeginPlay)

(fn ConstructionScript)
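; Flamethrower weapon that registers and equips itself on the player at BeginPlay and toggles a Niagara flame on Fire and EndFire.
; A trigger zone tracks overlapping actors that implement BPI_FlammeThrower.
; Niagara targets the weapon as a callback object, and each ParticleData event damages every tracked actor, regardless of particle positions.
; Tick feeds age-scaled player velocity into the effect; an older sphere-trace damage path is left unconnected.
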(event OnComponentBeginOverlap(EnnemiesTriggerZone)
  (params (OverlappedComponent :type Primitive%20Component%20Object%20Reference) (OtherActor :type Actor%20Object%20Reference) (OtherComp :type Primitive%20Component%20Object%20Reference) (OtherBodyIndex :type Integer) (bFromSweep :type Boolean) (SweepResult :type Hit%20Result%20Structure%20%28by%20ref%29))
  (if (Utilities|DoesObjectImplementInterface OtherActor "/Game/Blueprint/weapon/BPI_FlammeThrower.BPI_FlammeThrower_C")
    (Utilities|Array|AddUnique (Variables|Default|GetEnnemiesInRanged) OtherActor)))

(event OnComponentEndOverlap(EnnemiesTriggerZone)
  (params (OverlappedComponent :type Primitive%20Component%20Object%20Reference) (OtherActor :type Actor%20Object%20Reference) (OtherComp :type Primitive%20Component%20Object%20Reference) (OtherBodyIndex :type Integer))
  (Utilities|Array|RemoveItem (Variables|Default|GetEnnemiesInRanged) OtherActor))

(event Custom|FireLineTrace)

(event EventTick
  (params (DeltaSeconds :type Float%20%28single-precision%29))
  (bind _niagara (Variables|Default|GetNiagara))
  (Class|NiagaraComponent|SetNiagaraVariableVec3 _niagara "PlayerVelocity" (* (Transformation|GetVelocity (Variables|Default|GetplayerRef)) (Math|Float|NormalizetoRange (Class|NiagaraComponent|GetDesiredAge _niagara) 1.0 1.5))))

(event EventParticleData
  (params (Data :type Array%20of%20Basic%20Particle%20Data%20Structures) (NiagaraSystem :type Niagara%20System%20Object%20Reference) (SimulationPositionOffset :type Vector%20%28by%20ref%29 :default "0, 0, 0"))
  (for _array_element (Variables|Default|GetEnnemiesInRanged)
    (Game|Damage|ApplyDamage _array_element (Variables|Default|GetFireDamage) 0 0)
    (Development|PrintString "Hello" true true "(R=0.000000,G=0.660000,B=1.000000,A=1.000000)" 0.0)))

(event EventEndFire
  ;[0.01096 0.01161 0.0137] Collision feu niagara
  (Components|Activation|Deactivate (Variables|Default|GetNiagara))
  (Utilities|Time|ClearandInvalidateTimerbyHandle (Variables|Default|GetFireTrace)))

(event EventFire
  ;[0.01096 0.01161 0.0137] Collision feu niagara
  (Components|Activation|Activate (Variables|Default|GetNiagara) true))

(event EventBeginPlay
  (bind _playerref (Variables|Default|GetplayerRef)
    (:then
      (Utilities|Array|AddUnique (Variables|/Game/ThirdPerson/Blueprints/BP_ThirdPersonCharacter.BP_ThirdPersonCharacter_C|GetWeaponsTab _playerref) self)
      (Default|EquipWeapon _playerref self)
      (Class|NiagaraComponent|SetVariableObject (Variables|Default|GetNiagara) "Target" self))
    (:else)))

(fn ConstructionScript
  (|CallParentFunction)
  (Transformation|SetRelativeLocation (Variables|Default|GetNiagara) (Variables|/Script/Engine.SceneComponent|GetRelativeLocation (Variables|Default|GetProjectileSpawn)) false false))
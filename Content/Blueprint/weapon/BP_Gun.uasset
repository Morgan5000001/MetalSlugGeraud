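; BP_Gun is an automatic weapon that equips itself to its referenced player on BeginPlay and fires projectiles.
; Fire starts a looping timer, gated by CanShoot, whose negative initial delay cancels the wait before the first shot.
; Each tick spawns a BP_Projectile at the ProjectileSpawn component and overrides its movement velocity.
; EndFire clears the timer and re-enables shooting.
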(event Custom|Shoot
  (bind _returnvalue (Game|SpawnActorfromClass "/Game/Blueprint/Projectile/BP_Projectile.BP_Projectile_C" (Transformation|GetWorldTransform (Variables|Default|GetProjectileSpawn)) "Undefined" "MultiplyWithRoot" 0 0))
  (Variables|/Script/Engine.MovementComponent|SetVelocity (Variables|/Game/Blueprint/Projectile/BP_Projectile.BP_Projectile_C|GetProjectileMovement _returnvalue) (Variables|Default|GetVelocity)))

(event EventBeginPlay
  (bind _playerref (Variables|Default|GetplayerRef)
    (:then
      (Default|EquipWeapon _playerref self)
      (Development|PrintString "equip trigger"))
    (:else)))

(event EventFire
  (if (Variables|Default|GetCan%20Shoot)
    (Variables|Default|SetCan%20Shoot false)
    (bind _returnvalue (Utilities|Time|SetTimerbyEvent (delegate Custom|Shoot) 0.2 true -0.2))
    (Variables|Default|SetFireTimer _returnvalue)))

(event EventEndFire
  (Variables|Default|SetCan%20Shoot true)
  (Utilities|Time|ClearandInvalidateTimerbyHandle (Variables|Default|GetFireTimer)))

(fn ConstructionScript
  (|CallParentFunction))
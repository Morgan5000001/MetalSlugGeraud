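; BP_Sword is a melee weapon that swings on Fire and damages what it hits in front of the third-person character.
; A DoOnce blocks repeat attacks until the montage completes, and a timer calls the swing, which alternates between two root attack montages via FlipFlop.
; A montage notify runs a debug-drawn, stationary sphere trace ahead of the character, applying fixed damage only to actors implementing BPI_FlammeThrower.
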(event Custom|BoolAcivate
  (bind _as_bp_third_person_character (Variables|Default|GetAs%20BP%20Third%20Person%20Character))
  (bind _returnvalue (Transformation|GetActorLocation _as_bp_third_person_character))
  (bind _returnvalue_2 (Transformation|GetActorForwardVector _as_bp_third_person_character))
  (bind _returnvalue_3 (* _returnvalue_2 2e+02))
  (bind _returnvalue_4 (+ _returnvalue _returnvalue_3))
  (bind _isa (Utilities|FlowControl|FlipFlop)
    (:A
      _)
    (:B
      _))
  (Animation|Montage|PlayMontage (Variables|/Script/Engine.Character|GetMesh (Variables|Default|GetAs%20BP%20Third%20Person%20Character)) (select _isa "/Game/AnimAttackRoot_Montage.AnimAttackRoot_Montage" "/Game/AnimAttackRoot1_Montage.AnimAttackRoot1_Montage")
    (:OnCompleted
      (Utilities|FlowControl|DoOnce false) ; enters at Reset
    )
    (:OnNotifyBegin
      (bind (_outhit _returnvalue_5) (Collision|SphereTraceByChannel _returnvalue_4 _returnvalue_4 1e+02 "TraceTypeQuery1" false 0 "ForDuration"))
      (if _returnvalue_5
        (if (Utilities|DoesObjectImplementInterface (.HitActor (Collision|BreakHitResult _outhit)) "/Game/Blueprint/weapon/BPI_FlammeThrower.BPI_FlammeThrower_C")
          (Game|Damage|ApplyDamage (.HitActor (Collision|BreakHitResult _outhit)) 52.0 0 0))))))

(event EventBeginPlay
  (|CallParentFunction) ; This node is disabled and will not be called.\nDrag off pins to build functionality.
)

(event Collision|EventActorBeginOverlap
  (params (OtherActor :type Actor%20Object%20Reference)))

(event EventTick
  (params (DeltaSeconds :type Float%20%28single-precision%29)))

(event EventFire
  (Utilities|FlowControl|DoOnce false
    (:Completed
      (Utilities|Time|SetTimerbyEvent (delegate Custom|BoolAcivate) 2.0 false -2.0))))

(fn ConstructionScript
  (|CallParentFunction))
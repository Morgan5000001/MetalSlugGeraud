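; BP_Ammo is a collectible ammo pickup that spins slowly around its vertical axis.
; When the third-person character overlaps its Box, it adds a fixed amount of ammo to that character's current weapon, spawns a Niagara collect effect and destroys itself.
; The construction script gives the Tresor component a random mesh from the RandomMesh array, varying the pickup's appearance.
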(event OnComponentBeginOverlap(Box)
  (params (OverlappedComponent :type Primitive%20Component%20Object%20Reference) (OtherActor :type Actor%20Object%20Reference) (OtherComp :type Primitive%20Component%20Object%20Reference) (OtherBodyIndex :type Integer) (bFromSweep :type Boolean) (SweepResult :type Hit%20Result%20Structure%20%28by%20ref%29))
  (bind _asbp_third_person_character (Utilities|Casting|CastToBP_ThirdPersonCharacter OtherActor))
  (Variables|/Game/Blueprint/weapon/BP_WeaponParent.BP_WeaponParent_C|SetAmmo (Variables|/Game/ThirdPerson/Blueprints/BP_ThirdPersonCharacter.BP_ThirdPersonCharacter_C|GetCurrentWeapon _asbp_third_person_character) (+ (Variables|/Game/Blueprint/weapon/BP_WeaponParent.BP_WeaponParent_C|GetAmmo (Variables|/Game/ThirdPerson/Blueprints/BP_ThirdPersonCharacter.BP_ThirdPersonCharacter_C|GetCurrentWeapon _asbp_third_person_character)) 10))
  (Niagara|SpawnSystematLocation "/Game/Niagara/NS_Collect.NS_Collect" (Transformation|GetActorLocation))
  (Actor|DestroyActor))

(event EventBeginPlay)

(event EventTick
  (params (DeltaSeconds :type Float%20%28single-precision%29))
  (Class|Actor|AddActorWorldRotation (Math|Rotator|MakeRotator 0.0 0.0 (* DeltaSeconds 5e+01))))

(fn ConstructionScript
  (Components|StaticMesh|SetStaticMesh (Variables|Default|GetTresor) (.OutItem (Utilities|Array|Random (Variables|Default|GetRandomMesh)))))
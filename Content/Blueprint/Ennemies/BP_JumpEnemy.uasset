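; BP_JumpEnemy is an enemy that leaps onto the player's head and explodes after a delay.
; Its detection box triggers a one-time jump, with the ToPlayer timeline lerping the mesh toward a point above the character's live position.
; On landing, it snaps onto the character's HeadSocket and starts a timer that applies damage, spawns an explosion effect and destroys the actor.
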(event OnComponentBeginOverlap(BoxDetectPlayer)
  (params (OverlappedComponent :type Primitive%20Component%20Object%20Reference) (OtherActor :type Actor%20Object%20Reference) (OtherComp :type Primitive%20Component%20Object%20Reference) (OtherBodyIndex :type Integer) (bFromSweep :type Boolean) (SweepResult :type Hit%20Result%20Structure%20%28by%20ref%29))
  (bind _asbp_third_person_character (Utilities|Casting|CastToBP_ThirdPersonCharacter OtherActor))
  (Utilities|FlowControl|DoOnce false
    (:Completed
      (CallFunction|JumptoPlayer _asbp_third_person_character))))

(event Custom|JumpToPlayer
  (params (As%20BP%20Third%20Person%20Character :type BP%20Third%20Person%20Character%20Object%20Reference))
  (bind _returnvalue (Transformation|GetActorLocation As%20BP%20Third%20Person%20Character))
  (bind _newtrack_0 (Timeline|ToPlayer PlayFromStart)
    (:Update
      (Transformation|SetRelativeLocation (Variables|Default|GetStaticMesh) (Math|Vector|Lerp(Vector) (Variables|/Script/Engine.SceneComponent|GetRelativeLocation (Variables|Default|GetStaticMesh)) (Math|Vector|MakeVector (.x _returnvalue) (.y _returnvalue) (+ (.z _returnvalue) 5e+01)) _newtrack_0) true false))
    (:Finished
      (Transformation|SetRelativeLocation (Variables|Default|GetStaticMesh) "0.000000,10.000000,10.000000" false false)
      (Transformation|AttachComponentToComponent (Variables|/Script/Engine.Character|GetMesh As%20BP%20Third%20Person%20Character) "HeadSocket" "SnapToTarget" "SnapToTarget" "SnapToTarget" true)
      (Utilities|Time|SetTimerbyEvent (delegate Custom|CustomEvent) (Variables|Default|GetCdDestroy)))))

(event Custom|CustomEvent
  (Game|Damage|ApplyDamage (stale Custom|JumpToPlayer As%20BP%20Third%20Person%20Character) 1.0 0 0)
  (Niagara|SpawnSystematLocation "/Game/Niagara/FX_ExplosionLethalCompany.FX_ExplosionLethalCompany" (Transformation|GetWorldLocation (Variables|Default|GetStaticMesh)))
  (Actor|DestroyActor))

(event EventBeginPlay
  (Components|Timeline|SetPlayRate (Variables|Default|GetLoopIdle) 2.0))

(event Collision|EventActorBeginOverlap
  (params (OtherActor :type Actor%20Object%20Reference)))

(event EventTick
  (params (DeltaSeconds :type Float%20%28single-precision%29)))

(fn ConstructionScript)
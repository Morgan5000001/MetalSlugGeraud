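; Parent enemy Blueprint that tracks HP, handles death and awards score to the player.
; Damage lowers HP; at zero, a one-time branch flags death, adds points to the third-person character, plays a death montage, deactivates movement and destroys the actor on montage notify end.
; Tick prints HP and, when the player is seen, computes and prints the look-at pitch toward them.
; Attack and Shoot are empty stubs.
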(event Custom|Attack)

(event Custom|Score
  (bind _returnvalue (Game|GetPlayerCharacter 0))
  (bind _asbp_third_person_character (Utilities|Casting|CastToBP_ThirdPersonCharacter _returnvalue))
  (Variables|/Game/ThirdPerson/Blueprints/BP_ThirdPersonCharacter.BP_ThirdPersonCharacter_C|SetScore _asbp_third_person_character (+ (Variables|Default|GetScor) (Variables|/Game/ThirdPerson/Blueprints/BP_ThirdPersonCharacter.BP_ThirdPersonCharacter_C|GetScore _asbp_third_person_character))))

(event Game|Damage|EventAnyDamage
  (params (Damage :type Float%20%28single-precision%29) (DamageType :type Damage%20Type%20Object%20Reference) (InstigatedBy :type Controller%20Object%20Reference) (DamageCauser :type Actor%20Object%20Reference))
  (bind _output_get (Variables|Default|SetHP (- (Variables|Default|GetHP) Damage)))
  (if (<= _output_get 0.0)
    (Utilities|FlowControl|DoOnce false
      (:Completed
        (Variables|Default|SetDead? true)
        (CallFunction|Score)
        (Animation|Montage|PlayMontage (Variables|Character|GetMesh) "/Game/AnimMagedead_Montage.AnimMagedead_Montage"
          (:then
            (Components|Activation|Deactivate (Variables|Character|GetCharacterMovement)))
          (:OnNotifyEnd
            (Actor|DestroyActor)))))))

(event EventTick
  (params (DeltaSeconds :type Float%20%28single-precision%29))
  (Development|PrintString (Utilities|String|ToString(Float) (Variables|Default|GetHP)) true true "(R=0.000000,G=0.660000,B=1.000000,A=1.000000)" 0.0)
  (if (Variables|Default|GetIsSee?)
    (bind _output_get (Variables|Default|SetValueFindPlayer (.pitch (Math|Rotator|FindLookatRotation (Transformation|GetActorLocation) (Transformation|GetActorLocation (Game|GetPlayerCharacter 0))))))
    (Development|PrintString (Utilities|String|ToString(Float) _output_get) true true "(R=0.000000,G=0.660000,B=1.000000,A=1.000000)" 0.0)))

(fn ConstructionScript)

(fn Shoot)
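; BP_PtndeOneWay is a one-way platform for BP_ThirdPersonCharacter, switching its StaticMesh collision based on trigger overlaps.
; Entering Dessous (below) disables collision.
; Entering Dessus (above) enables collision if the character's IsUp is set, and leaving it disables collision if IsDown is set.
; Leaving Dessous only casts the actor, and collision changes apply to the whole mesh rather than per character.
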(event OnComponentBeginOverlap(Dessus)
  (params (OverlappedComponent :type Primitive%20Component%20Object%20Reference) (OtherActor :type Actor%20Object%20Reference) (OtherComp :type Primitive%20Component%20Object%20Reference) (OtherBodyIndex :type Integer) (bFromSweep :type Boolean) (SweepResult :type Hit%20Result%20Structure%20%28by%20ref%29))
  (bind _asbp_third_person_character (Utilities|Casting|CastToBP_ThirdPersonCharacter OtherActor))
  (if (Variables|/Game/Blueprints/Player/BP_ThirdPersonCharacter.BP_ThirdPersonCharacter_C|GetIsUp? _asbp_third_person_character)
    (Collision|SetCollisionEnabled (Variables|Default|GetStaticMesh) "QueryAndPhysics")))

(event OnComponentEndOverlap(Dessus)
  (params (OverlappedComponent :type Primitive%20Component%20Object%20Reference) (OtherActor :type Actor%20Object%20Reference) (OtherComp :type Primitive%20Component%20Object%20Reference) (OtherBodyIndex :type Integer))
  (bind _asbp_third_person_character (Utilities|Casting|CastToBP_ThirdPersonCharacter OtherActor))
  (if (Variables|/Game/Blueprints/Player/BP_ThirdPersonCharacter.BP_ThirdPersonCharacter_C|GetIsDown _asbp_third_person_character)
    (Collision|SetCollisionEnabled (Variables|Default|GetStaticMesh) "NoCollision")))

(event OnComponentBeginOverlap(Dessous)
  (params (OverlappedComponent :type Primitive%20Component%20Object%20Reference) (OtherActor :type Actor%20Object%20Reference) (OtherComp :type Primitive%20Component%20Object%20Reference) (OtherBodyIndex :type Integer) (bFromSweep :type Boolean) (SweepResult :type Hit%20Result%20Structure%20%28by%20ref%29))
  (Utilities|Casting|CastToBP_ThirdPersonCharacter OtherActor)
  (Collision|SetCollisionEnabled (Variables|Default|GetStaticMesh) "NoCollision"))

(event OnComponentEndOverlap(Dessous)
  (params (OverlappedComponent :type Primitive%20Component%20Object%20Reference) (OtherActor :type Actor%20Object%20Reference) (OtherComp :type Primitive%20Component%20Object%20Reference) (OtherBodyIndex :type Integer))
  (Utilities|Casting|CastToBP_ThirdPersonCharacter OtherActor))

(event EventBeginPlay)

(event Collision|EventActorBeginOverlap
  (params (OtherActor :type Actor%20Object%20Reference)))

(event EventTick
  (params (DeltaSeconds :type Float%20%28single-precision%29)))

(fn ConstructionScript)